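; Trap ball actor that rolls as a hazard and ends the game in defeat when its sphere hits something.
; Tick pushes the physics Sphere along -X with a mass-independent force.
; Any hit, without checking the other actor, ragdolls player 0, disables input, shows the BP_결과화면위젯 result widget as a loss, then destroys the ball.
; The delayed XZ-plane constraint is unconnected and never runs.
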(event `self.ReceiveBeginPlay`)

(event `self.ReceiveTick`
  (params (DeltaSeconds :type "Float (single-precision)"))
  (`PrimitiveComponent.AddForce` (`self.Sphere`) (-60.0 0.0 0.0) "None" true))

(event `self.Sphere.OnComponentHit`
  (params (HitComponent :type "PrimitiveComponent Object Reference") (OtherActor :type "Actor Object Reference") (OtherComp :type "PrimitiveComponent Object Reference") (NormalImpulse :type "Vector Structure") (Hit :type "HitResult Structure (by ref)"))
  (`self.playerDead`)
  (bind _returnvalue (`|CreateWidget` "/Game/시작해요언리얼/Blueprints/BP_결과화면위젯.BP_결과화면위젯_C"))
  (`UserWidget.AddToViewport` _returnvalue 0)
  (`self.DisableInput` (`GameplayStatics.GetPlayerCharacter` 0) (`GameplayStatics.GetPlayerController` 0))
  (`WidgetBlueprintLibrary.SetInputMode_UIOnlyEx` (`GameplayStatics.GetPlayerController` 0) null)
  (`/Game/시작해요언리얼/Blueprints/BP_결과화면위젯.SetResult` _returnvalue false)
  (`self.K2_DestroyActor`))

(fn `playerDead`
  (bind _returnvalue (`GameplayStatics.GetPlayerCharacter` 0))
  (bind _mesh (`Character.Mesh` _returnvalue))
  (`/Engine/EditorBlueprintResources/StandardMacros.IsValid` _returnvalue
    (:`Is Valid`
      (`PrimitiveComponent.SetCollisionEnabled` (`Character.CapsuleComponent` _returnvalue) "NoCollision")
      (`CharacterMovementComponent.SetMovementMode` (`Character.CharacterMovement` _returnvalue) "MOVE_None" 0)
      (`PrimitiveComponent.SetCollisionProfileName` _mesh "Ragdoll" true)
      (`SkeletalMeshComponent.SetAllBodiesSimulatePhysics` _mesh true))))

(fn `UserConstructionScript`)