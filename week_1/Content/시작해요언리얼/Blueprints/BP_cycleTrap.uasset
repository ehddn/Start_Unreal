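; BP_cycleTrap is a moving trap actor whose Sphere component circles continuously on a horizontal elliptical path, with no overlap or damage logic in its graphs.
; Each Tick sets the Sphere's relative location from degree-based cosine and sine of Time, scaled by RadiusX and RadiusY.
; Time advances by delta seconds times Speed and resets to zero at 360.
; Tick also re-applies the root's own world location to the actor.
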(event `self.ReceiveTick`
  (params (DeltaSeconds :type "Float (single-precision)"))
  (bind _time (`self.Time`))
  (bind _returnvalue (+ (* (`GameplayStatics.GetWorldDeltaSeconds`) (`self.Speed`)) (`self.Time`)))
  (`self.K2_SetActorLocation` (`SceneComponent.K2_GetComponentLocation` (`self.DefaultSceneRoot`)))
  (`SceneComponent.K2_SetRelativeLocation` (`self.Sphere`) (`KismetMathLibrary.MakeVector` (* (`KismetMathLibrary.DegCos` _time) (`self.RadiusX`)) (* (`KismetMathLibrary.DegSin` _time) (`self.RadiusY`))) false false)
  (if (>= _returnvalue 360.0)
    (set `self.Time` 0.0)
    (else
      (set `self.Time` _returnvalue))))

(fn `UserConstructionScript`)